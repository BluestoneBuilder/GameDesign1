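; BP_Door is a security door for the stealth game that shows its required level as color-coded text on two text renders.
; On box overlap, it compares the custom third-person character's SecurityLevel to NeededSecurityLevel.
; If sufficient, it plays a sound and a timeline slides the actor upward once; otherwise it prints the needed level.
; Despite a "Remove a Key" comment, opening leaves SecurityLevel unchanged.
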(event `self.ReceiveBeginPlay`
  (bind _doorcolor (`self.DoorColor`))
  (bind _returnvalue (`KismetTextLibrary.Conv_IntToText` (`self.NeededSecurityLevel`)))
  (`TextRenderComponent.K2_SetText` (`self.TextRender`) _returnvalue)
  (`TextRenderComponent.K2_SetText` (`self.TextRender1`) _returnvalue)
  (switch `int` (`self.NeededSecurityLevel`)
    (:`0`
      (set `self.DoorColor` (`self.Level 0 Color`)))
    (:`1`
      (set `self.DoorColor` (`self.Level 1 Color`)))
    (:`2`
      (set `self.DoorColor` (`self.Level 2 Color`)))
    (:`3`
      (set `self.DoorColor` (`self.Level 3 Color`)))
    (:`4`
      (set `self.DoorColor` (`self.Level 4 Color`))))
  (`TextRenderComponent.SetTextRenderColor` (`self.TextRender`) _doorcolor)
  (`TextRenderComponent.SetTextRenderColor` (`self.TextRender1`) _doorcolor))

(event `self.Box collision.OnComponentBeginOverlap`
  (params (OverlappedComponent :type "PrimitiveComponent Object Reference") (OtherActor :type "Actor Object Reference") (OtherComp :type "PrimitiveComponent Object Reference") (OtherBodyIndex :type Integer) (bFromSweep :type Boolean) (SweepResult :type "HitResult Structure (by ref)"))
  (bind (_returnvalue_x _returnvalue_y _returnvalue_z) (`KismetMathLibrary.BreakVector` (`self.K2_GetActorLocation`)))
  (bind _asbp_third_person_character_custom (cast `/Game/StealthGame/Core/Characters/PlayerCharacter/BP_ThirdPersonCharacterCustom` OtherActor))
  (bind _securitylevel (`/Game/StealthGame/Core/Characters/PlayerCharacter/BP_ThirdPersonCharacterCustom.SecurityLevel` _asbp_third_person_character_custom))
  (if (>= _securitylevel (`self.NeededSecurityLevel`))
    (`/Engine/EditorBlueprintResources/StandardMacros.DoOnce` false
      (:`Completed`
        (set `/Game/StealthGame/Core/Characters/PlayerCharacter/BP_ThirdPersonCharacterCustom.SecurityLevel` _securitylevel _asbp_third_person_character_custom) ; Remove a Key, then open door.
        (`AudioComponent.Play` (`self.DoorOpenSound`) 0.0)
        (bind _output_get (set `self.StartLocation` _returnvalue_z))
        (bind (_direction _doorrotation) (`Timeline|DoorOpen`)
          (:`Update`
            (`self.K2_SetActorLocation` (`KismetMathLibrary.MakeVector` _returnvalue_x _returnvalue_y (+ (* _doorrotation 200.0) _output_get)))))))
    (else
      (`KismetSystemLibrary.PrintString` (`KismetStringLibrary.Concat_StrStr` "Need security level " (`KismetStringLibrary.Conv_IntToString` (`self.NeededSecurityLevel`))) true true (struct :`R` 0.479167 :`G` 0.051103 :`A` 1.0) 5.0))))

(fn `UserConstructionScript`)