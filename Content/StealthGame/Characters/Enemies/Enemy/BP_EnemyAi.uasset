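; Stealth enemy AI character that patrols, investigates noises, and chases and attacks the player.
; PawnSensing sets player visibility with a retriggerable timeout, driving an awareness timer on Tick that halts the enemy, then starts a chase once full.
; Otherwise it follows patrol points, wanders randomly or returns to its start via AIMoveTo.
; Melee attacks sphere-trace from the hand, reload the player's checkpoint on hit and repeat while hostile.
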(event `self.ReceiveTick`
  (params (DeltaSeconds :type "Float (single-precision)"))
  (`|ExecutionSequence`
    (:`then_0`
      ; Change awareness value if player is visible
      (if (`self.bPlayerVisible`)
        (if (< (`self.fAwareness`) (`self.fEnemySpotPlayerTime`))
          (set `self.fAwareness` (+ (`self.fAwareness`) DeltaSeconds))
          (else
            (set `self.fAwareness` (`self.fEnemySpotPlayerTime`))))
        (elif (> (`self.fAwareness`) 0.0)
          (set `self.fAwareness` (- (`self.fAwareness`) DeltaSeconds))
          (else
            (set `self.fAwareness` 0.0)))))
    (:`then_1`
      ; Check if player is fully spotted
      (if (>= (`self.fAwareness`) (`self.fEnemySpotPlayerTime`))
        ; Player Spotted
        (`self.ChasePlayer`)
        (else
          ; Player NOT spotted
          (if (`self.bPlayerVisible`)
            (`self.StopMovement`)
            (elif (`self.bCanMove`)
              (if (> (`KismetArrayLibrary.Array_Length` (`self.PatrolTargetPoints`)) 0)
                (if (`self.bTargetPointMovement`)
                  (`self.MoveToNextPatrolPoint`)
                  (else
                    (`self.PatrolRandom`)))
                (else
                  (`self.ReturnToStartPosition`))))))))))

(event `self.ReceiveBeginPlay`
  (set `self.StartPosition` (`self.K2_GetActorLocation`))
  (set `self.StartRotation` (`self.K2_GetActorRotation`)))

(event `self.PawnSensing.OnSeePawn`
  (params (Pawn :type "Pawn Object Reference"))
  (cast `/Game/StealthGame/Core/Characters/PlayerCharacter/BP_ThirdPersonCharacterCustom` Pawn
    (:`then`
      (`|ExecutionSequence`
        (:`then_0`
          (`KismetSystemLibrary.PrintString` "Is someone there?" true true (struct :`R` 1.0 :`G` 0.988249 :`B` 0.100228 :`A` 1.0))
          (set `self.bPlayerVisible` true))
        (:`then_1`
          (`KismetSystemLibrary.RetriggerableDelay` 1.0)
          (set `self.bPlayerVisible` false :!label _label))))
    (:`CastFailed`
      (goto _label))))

(event `ChasePlayer`
  (`self.UpdateWalkSpeed` (`self.fChaseWalkSpeed`))
  (`KismetSystemLibrary.PrintString` "I'm gonna get you" true true (struct :`R` 1.0 :`G` 0.149976 :`B` 0.035568 :`A` 1.0))
  (set `self.bCanMove` false)
  (`|AIMoveTo` self (0.0 0.0 0.0) (`GameplayStatics.GetPlayerCharacter` 0) 75.0
    (:`OnSuccess`
      (`self.Attack`)
      (`KismetSystemLibrary.PrintString` "Bonk")
      (set `self.bCanMove` true))))

(event `PatrolRandom`
  (`self.UpdateWalkSpeed` (`self.fPatrolWalkSpeed`))
  (set `self.bCanMove` false)
  (`|AIMoveTo` self (`NavigationSystemV1.K2_GetRandomReachablePointInRadius` (`self.K2_GetActorLocation`) (`self.fRandomPatrolRadius`) null null) null 75.0
    (:`OnSuccess`
      (`KismetSystemLibrary.Delay` 3.0)
      (set `self.bCanMove` true))))

(event `StopMovement`
  (`self.UpdateWalkSpeed` 0.0)
  (`|AIMoveTo` null (`self.K2_GetActorLocation`) null
    (:`then`
      (set `self.bCanMove` true))))

(event `ReturnToStartPosition`
  (`self.UpdateWalkSpeed` (`self.fPatrolWalkSpeed`))
  (set `self.bCanMove` false)
  (`|AIMoveTo` self (`self.StartPosition`) null 75.0
    (:`OnSuccess`
      (`self.K2_SetActorRotation` (`self.StartRotation`))
      (`KismetSystemLibrary.Delay` 3.0)
      (set `self.bCanMove` true))))

(event `MoveToNextPatrolPoint`
  (`self.UpdateWalkSpeed` (`self.fPatrolWalkSpeed`))
  (set `self.bCanMove` false)
  (`|AIMoveTo` self (0.0 0.0 0.0) (`|GetArrayItem` (`self.PatrolTargetPoints`) (`self.PatrolTargetPointIndex`)) 75.0
    (:`OnSuccess`
      (`self.SetNextPatrolPointIndex`)
      (`KismetSystemLibrary.Delay` 3.0)
      (set `self.bCanMove` true))))

(event `SetNextPatrolPointIndex`
  (set `self.PatrolTargetPointIndex` (mod (+ (`self.PatrolTargetPointIndex`) 1) (`KismetArrayLibrary.Array_Length` (`self.PatrolTargetPoints`)))))

(event `self.PawnSensing.OnHearNoise`
  (params (Instigator :type "Pawn Object Reference") (Location :type "Vector Structure (by ref)") (Volume :type "Float (single-precision)"))
  (`self.UpdateWalkSpeed` (`self.fInvestigateWalkSpeed`))
  (set `self.bCanMove` false)
  (`|AIMoveTo` self Location Instigator 75.0
    (:`OnSuccess`
      (`self.SetNextPatrolPointIndex`)
      (`KismetSystemLibrary.Delay` 6.0) ; Rock distraction amount
      (set `self.bCanMove` true))))

(event `Attack`
  (bind _returnvalue (`SceneComponent.GetSocketLocation` (`self.Mesh`) "hand_r"))
  ;[0.15 0.1407 0.04319 0.5] Bonk
  (`/Engine/EditorBlueprintResources/StandardMacros.DoOnce` false :!label _label_2 ; Only Reset Attack on miss.
    (:`Completed`
      (bind _notifyname (`|PlayMontage` (`self.Mesh`) "/Game/StealthGame/Characters/Enemies/Enemy/AM_Attack_01.AM_Attack_01") ; Play the AM_Attack_01
        (:`then`
          (`KismetSystemLibrary.Delay` 0.45)
          (`KismetSystemLibrary.PrintString` "I'm attacking!")
          (bind (_outhits _returnvalue_2) (`KismetSystemLibrary.SphereTraceMultiForObjects` :`Start` _returnvalue :`End` (+ _returnvalue (* (`self.GetActorForwardVector`) (`self.MeleeTraceDistance`))) :`Radius` (`self.MeleeTraceRadius`) :`ObjectTypes` (`|MakeArray` "ObjectTypeQuery3" :!type "EObjectTypeQuery Enum") :`DrawDebugType` "ForDuration")) ; Trace forward from hand socket.
          (if _returnvalue_2
            (for _array_element _outhits
              (bind _asbp_third_person_character_custom (cast `/Game/StealthGame/Core/Characters/PlayerCharacter/BP_ThirdPersonCharacterCustom` (`.HitActor` (`GameplayStatics.BreakHitResult` _array_element))))
              (`/Game/StealthGame/Core/Characters/PlayerCharacter/BP_ThirdPersonCharacterCustom.LoadCheckpoint` _asbp_third_person_character_custom)
              (set `self.bHostile` false) ; ...and stop attacking...
            )))
        (:`OnCompleted`
          (if (`self.bHostile`)
            (`self.ResetAttack`)))))))

(event `ResetAttack`
  ;[0.15 0.1407 0.04319 0.5] Bonk
  (goto _label_2 :!via `Reset`))

(fn `UpdateWalkSpeed`
  (params (NewWalkSpeed :type "Float (double-precision)" :default 600.0))
  (set `CharacterMovementComponent.MaxWalkSpeed` NewWalkSpeed (`self.CharacterMovement`)))

(fn `UserConstructionScript`)