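; Stealth-game security camera that spots the player and alerts enemies by making a noise at the player's location.
; Sight events set a visibility flag, cleared by a retriggerable delay once sightings stop.
; A looping half-second timer raises or decays clamped awareness, tinting the spotlight white, amber or red.
; At the threshold, a DoOnce fires the noise, caught audio and debug sphere, re-arming when sight is lost.
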(event `self.ReceiveBeginPlay`
  (`self.Awareness` :!label _label)
  (`KismetSystemLibrary.Delay` 0.5)
  (goto _label))

(event `self.CameraSight.OnSeePawn`
  (params (Pawn :type "Pawn Object Reference"))
  (cast `/Game/StealthGame/Core/Characters/PlayerCharacter/BP_ThirdPersonCharacterCustom` Pawn
    (:`then`
      (`|ExecutionSequence`
        (:`then_0`
          (set `self.CanSeePlayer` true))
        (:`then_1`
          (`KismetSystemLibrary.RetriggerableDelay` 0.6)
          (set `self.CanSeePlayer` false))))
    (:`CastFailed`
      (set `self.CanSeePlayer` false))))

(event `Awareness`
  (bind (_returnvalue_x _returnvalue_y) (`KismetMathLibrary.BreakVector` (`self.K2_GetActorLocation` (`GameplayStatics.GetPlayerCharacter` 0))))
  (if (`self.CanSeePlayer`)
    (`LightComponent.SetLightColor` (`self.SpotLight`) (struct :`R` 1.0 :`G` 0.670833 :`B` 0.081226 :`A` 1.0) true)
    (set `self.CamAwareness` (`KismetMathLibrary.Clamp` (+ (`self.CamAwareness`) 1) 0 (`self.CamSpottedThreshold`)))
    (if (>= (`self.CamAwareness`) (`self.CamSpottedThreshold`))
      (`LightComponent.SetLightColor` (`self.SpotLight`) (struct :`R` 1.0 :`B` 0.032337 :`A` 1.0) true)
      (`/Engine/EditorBlueprintResources/StandardMacros.DoOnce` false :!label _label_2
        (:`Completed`
          (`PawnNoiseEmitterComponent.MakeNoise` (`self.CamEnemyNotify`) self 1.0 (`KismetMathLibrary.MakeVector` _returnvalue_x _returnvalue_y))
          (`AudioComponent.Play` (`self.CamCaughtAudio`) 0.0)
          (`KismetSystemLibrary.DrawDebugSphere` (`KismetMathLibrary.MakeVector` _returnvalue_x _returnvalue_y) 100.0 12 (struct :`R` 1.0 :`G` 1.0 :`B` 1.0 :`A` 1.0) 0.6))))
    (else
      (`|ExecutionSequence`
        (:`then_0`
          (set `self.CamAwareness` (`KismetMathLibrary.Clamp` (- (`self.CamAwareness`) 1) 0 (`self.CamSpottedThreshold`)))
          (if (<= (`self.CamAwareness`) 0)
            (`LightComponent.SetLightColor` (`self.SpotLight`) (struct :`R` 1.0 :`G` 1.0 :`B` 1.0 :`A` 1.0) true)))
        (:`then_1`
          (goto _label_2 :!via `Reset`))))))

(fn `UserConstructionScript`)