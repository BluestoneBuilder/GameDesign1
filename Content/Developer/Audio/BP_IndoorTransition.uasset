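; BP_IndoorTransition is a trigger actor in the audio developer folder that tells the custom third-person character when it moves indoors or outdoors.
; Overlapping InsideBox calls GoInside and overlapping OutisdeBox calls GoOutside, each printing a debug message.
; Each call runs only if the character's IsInside flag shows the opposite state, so repeated overlaps on one side do not retrigger it.
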(event `self.OutisdeBox.OnComponentBeginOverlap`
  (params (OverlappedComponent :type "PrimitiveComponent Object Reference") (OtherActor :type "Actor Object Reference") (OtherComp :type "PrimitiveComponent Object Reference") (OtherBodyIndex :type Integer) (bFromSweep :type Boolean) (SweepResult :type "HitResult Structure (by ref)"))
  (bind _asbp_third_person_character_custom (cast `/Game/StealthGame/Core/Characters/PlayerCharacter/BP_ThirdPersonCharacterCustom` OtherActor))
  (`KismetSystemLibrary.PrintText` "Out")
  (if (`/Game/StealthGame/Core/Characters/PlayerCharacter/BP_ThirdPersonCharacterCustom.isInside` _asbp_third_person_character_custom)
    (`/Game/StealthGame/Core/Characters/PlayerCharacter/BP_ThirdPersonCharacterCustom.GoOutside` _asbp_third_person_character_custom)))

(event `self.InsideBox.OnComponentBeginOverlap`
  (params (OverlappedComponent :type "PrimitiveComponent Object Reference") (OtherActor :type "Actor Object Reference") (OtherComp :type "PrimitiveComponent Object Reference") (OtherBodyIndex :type Integer) (bFromSweep :type Boolean) (SweepResult :type "HitResult Structure (by ref)"))
  (bind _asbp_third_person_character_custom (cast `/Game/StealthGame/Core/Characters/PlayerCharacter/BP_ThirdPersonCharacterCustom` OtherActor))
  (`KismetSystemLibrary.PrintString` "In")
  (if (not (`/Game/StealthGame/Core/Characters/PlayerCharacter/BP_ThirdPersonCharacterCustom.isInside` _asbp_third_person_character_custom))
    (`/Game/StealthGame/Core/Characters/PlayerCharacter/BP_ThirdPersonCharacterCustom.GoInside` _asbp_third_person_character_custom)))

(fn `UserConstructionScript`)